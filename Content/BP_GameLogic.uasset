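; BP_GameLogic runs a one-dimensional, Sokoban-style push puzzle on the FieldObjects enum array.
; BeginPlay adds the input mapping context, and IA_Horizontal finds the player's index and passes it with the truncated axis value to MoveObject.
; MoveObject recursively pushes chains of blocking objects, moving only when the chain stays within array bounds.
; PrintFieldObjects prints the array for debugging at start and after each input event.
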(event Input|EnhancedActionEvents|EnhancedInputActionIA_Horizontal
  (params (ActionValue :type Float%20%28double-precision%29) (ElapsedSeconds :type Float%20%28double-precision%29) (TriggeredSeconds :type Float%20%28double-precision%29) (InputAction :type Input%20Action%20Object%20Reference :default "/Game/IA_Horizontal.IA_Horizontal"))
  (bind _playerindex (CallFunction|GetPlayerIndex))
  (CallFunction|MoveObject _playerindex (Math|Float|Truncate ActionValue))
  (CallFunction|PrintFieldObjects))

(event EventBeginPlay
  (Input|AddMappingContext (PlayerController|LocalPlayerSubsystems|GetEnhancedInputLocalPlayerSubsystem (Game|GetPlayerController 0)) "/Game/IMC_lnGame.IMC_lnGame" 0 "(bIgnoreAllPressedKeysUntilRelease=True,bForceImmediately=False,bNotifyUserSettings=False)")
  (CallFunction|PrintFieldObjects))

(event Collision|EventActorBeginOverlap
  (params (OtherActor :type Actor%20Object%20Reference)))

(event EventTick
  (params (DeltaSeconds :type Float%20%28single-precision%29)))

(fn ConstructionScript)

(fn PrintFieldObjects
  (Variables|Default|SetDebugStgringBuffer "")
  (for _array_element (Variables|Default|GetFieldObjects)
    (Variables|Default|SetDebugStgringBuffer (Utilities|String|Append (Variables|Default|GetDebugStgringBuffer) "，" (Utilities|String|ToString(Integer) (Math|Conversions|ToInteger(Byte) _array_element)))))
  (Development|PrintString (Variables|Default|GetDebugStgringBuffer) true true "(R=0.000000,G=0.660000,B=1.000000,A=1.000000)" 3e+02 "PrintFieldObjects"))

(fn GetPlayerIndex
  (for (_array_element _array_index) (Variables|Default|GetFieldObjects)
    (if (Utilities|Enum|Equal(Enum) _array_element "NewEnumerator1")
      (return _array_index)))
  (return -1))

(fn MoveObject
  (params (MoveFromIndex :type Integer) (Velocity :type Integer))
  (bind _output_get (LocalVariables|SetMoveToIndex (+ MoveFromIndex Velocity)))
  (if (Utilities|Array|IsValidIndex (Variables|Default|GetFieldObjects) _output_get)
    (if (Utilities|Enum|NotEqual(Enum) (Utilities|Array|Get(acopy) (Variables|Default|GetFieldObjects) (LocalVariables|GetMoveToIndex)) "NewEnumerator2")
      _
      (else
        (bind _suceeded (CallFunction|MoveObject (LocalVariables|GetMoveToIndex) Velocity))
        (if _suceeded
          _
          (else
            (return false)))))
    (Utilities|Array|SetArrayElem (Variables|Default|GetFieldObjects) (LocalVariables|GetMoveToIndex) (Utilities|Array|Get(acopy) (Variables|Default|GetFieldObjects) MoveFromIndex))
    (Utilities|Array|SetArrayElem (Variables|Default|GetFieldObjects) MoveFromIndex "NewEnumerator0")
    (return true)
    (else
      (return false))))